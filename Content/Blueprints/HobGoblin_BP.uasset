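; HobGoblin enemy or creature Blueprint that continually flees from the player.
; On BeginPlay it caches the player's MainPaperCharacter and starts RunAway.
; RunAway uses AIMoveTo toward a point 500 units directly away from the player, keeping the goblin's own Z.
; Both success and failure re-trigger RunAway, forming an endless flee loop without Tick.
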(event Custom|RunAway
  (bind _returnvalue (Transformation|GetActorLocation))
  (bind _char_ref (Variables|Default|GetChar%20REF))
  (bind _returnvalue_2 (Transformation|GetActorLocation _char_ref))
  (bind _returnvalue_3 (Math|Rotator|FindLookatRotation _returnvalue _returnvalue_2))
  (bind _returnvalue_4 (Math|Vector|GetForwardVector _returnvalue_3))
  (bind _returnvalue_5 (* _returnvalue_4 "-500.000000,-500.000000,-500.000000"))
  (bind _returnvalue_6 (+ _returnvalue _returnvalue_5))
  (bind (_x _y) (Math|Vector|BreakVector _returnvalue_6))
  (AI|AIMoveTo self (Math|Vector|MakeVector _x _y (.Z (Math|Vector|BreakVector _returnvalue))) 0 5.0 false
    (:OnSuccess
      _)
    (:OnFail
      _))
  (CallFunction|RunAway))

(event EventBeginPlay
  (bind _asmain_paper_character (Utilities|Casting|CastToMainPaperCharacter (Game|GetPlayerCharacter 0)))
  (Variables|Default|SetChar%20REF _asmain_paper_character)
  (CallFunction|RunAway))

(event Collision|EventActorBeginOverlap
  (params (OtherActor :type Actor%20Object%20Reference)))

(event EventTick
  (params (DeltaSeconds :type Float%20%28single-precision%29)))

(fn ConstructionScript)